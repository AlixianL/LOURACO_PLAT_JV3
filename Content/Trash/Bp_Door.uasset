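; Bp_Door is a door actor that detects when the third-person player character enters or leaves its BoxDoor trigger.
; On overlap begin and end, it prints a debug message, casts to BP_ThirdPersonCharacter and sets that character's EnterIncolisionDoor flag to true or false.
; Both events also store the door as the character's DoorActor, so the reference remains after the character leaves.
; The graph contains no door movement or opening logic.
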(event `self.BoxDoor.OnComponentBeginOverlap`
  (params (OverlappedComponent :type "PrimitiveComponent Object Reference") (OtherActor :type "Actor Object Reference") (OtherComp :type "PrimitiveComponent Object Reference") (OtherBodyIndex :type Integer) (bFromSweep :type Boolean) (SweepResult :type "HitResult Structure (by ref)"))
  (`KismetSystemLibrary.PrintString` "Ty est dedans")
  (bind _asbp_third_person_character (cast `/Game/ThirdPerson/Blueprints/BP_ThirdPersonCharacter` OtherActor))
  (set `/Game/ThirdPerson/Blueprints/BP_ThirdPersonCharacter.EnterIncolisionDoor?` true _asbp_third_person_character)
  (set `/Game/ThirdPerson/Blueprints/BP_ThirdPersonCharacter.DoorActor` self _asbp_third_person_character))

(event `self.BoxDoor.OnComponentEndOverlap`
  (params (OverlappedComponent :type "PrimitiveComponent Object Reference") (OtherActor :type "Actor Object Reference") (OtherComp :type "PrimitiveComponent Object Reference") (OtherBodyIndex :type Integer))
  (`KismetSystemLibrary.PrintString` "Ty est Ou ?")
  (bind _asbp_third_person_character (cast `/Game/ThirdPerson/Blueprints/BP_ThirdPersonCharacter` OtherActor))
  (set `/Game/ThirdPerson/Blueprints/BP_ThirdPersonCharacter.EnterIncolisionDoor?` false _asbp_third_person_character)
  (set `/Game/ThirdPerson/Blueprints/BP_ThirdPersonCharacter.DoorActor` self _asbp_third_person_character))

(fn `UserConstructionScript`)